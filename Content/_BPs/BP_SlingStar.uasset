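; BP_SlingStar is a spinning star launcher that carries the player to a landing point on overlap.
; On BeginPlay, two timelines rotate its small and large star meshes.
; When the first-person character enters the collider, a timeline lerps their location from the Arrow component to the BP_SlingLanding found with GetActorOfClass.
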(event OnComponentBeginOverlap(Collider)
  (params (OverlappedComponent :type Primitive%20Component%20Object%20Reference) (OtherActor :type Actor%20Object%20Reference) (OtherComp :type Primitive%20Component%20Object%20Reference) (OtherBodyIndex :type Integer) (bFromSweep :type Boolean) (SweepResult :type Hit%20Result%20Structure%20%28by%20ref%29))
  (bind _returnvalue (Actor|GetActorOfClass "/Game/_BPs/BP_SlingLanding.BP_SlingLanding_C"))
  (Variables|Default|SetEndpoint _returnvalue)
  (bind _asbp_first_person_character (Utilities|Casting|CastToBP_FirstPersonCharacter OtherActor))
  (Variables|Default|Setcharref _asbp_first_person_character)
  (bind _alpha (Timeline|Move%20char PlayFromStart)
    (:Update
      (Transformation|SetActorTransform (Variables|Default|Getcharref) (Math|Transform|MakeTransform (Math|Vector|Lerp(Vector) (Transformation|GetWorldLocation (Variables|Default|GetArrow)) (Transformation|GetWorldLocation (Variables|/Script/Engine.Actor|GetRootComponent (Variables|Default|GetEndpoint))) _alpha) "0, 0, 0" "1.000000,1.000000,1.000000")))))

(event EventBeginPlay
  (Utilities|FlowControl|Sequence
    (:then_0
      (bind (_direction _y _z) (Timeline|Rotate%20small%20star PlayFromStart)
        (:Update
          (Transformation|SetRelativeRotation (Variables|Default|GetSmall_Star1) (Math|Rotator|MakeRotator 0.0 _z _y) false false))))
    (:then_1
      (bind (_direction_2 _y_2 _z_2) (Timeline|rotate%20big PlayFromStart)
        (:Update
          (Transformation|SetRelativeRotation (Variables|Default|GetLarge_Star1) (Math|Rotator|MakeRotator 0.0 _y_2 _z_2) false false))))))

(event Collision|EventActorBeginOverlap
  (params (OtherActor :type Actor%20Object%20Reference)))

(event EventTick
  (params (DeltaSeconds :type Float%20%28single-precision%29)))

(fn ConstructionScript)