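; BP_PipeEntrance4 is a Mario-style pipe entrance that teleports the first-person character to the BP_PipeExit4 actor in the level.
; On overlap it disables input and shrinks the player with a timeline, then moves them to the exit's Pipe2 location with the exit's rotation.
; A second timeline grows them back before input returns, while the character's ExitingPipe flag blocks re-entry during the trip.
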(event OnComponentBeginOverlap(Entrance)
  (params (OverlappedComponent :type Primitive%20Component%20Object%20Reference) (OtherActor :type Actor%20Object%20Reference) (OtherComp :type Primitive%20Component%20Object%20Reference) (OtherBodyIndex :type Integer) (bFromSweep :type Boolean) (SweepResult :type Hit%20Result%20Structure%20%28by%20ref%29))
  (bind _asbp_first_person_character (Utilities|Casting|CastToBP_FirstPersonCharacter OtherActor))
  (if (not (Variables|/Game/FirstPerson/Blueprints/BP_FirstPersonCharacter.BP_FirstPersonCharacter_C|GetExiting%20Pipe _asbp_first_person_character))
    (bind _output_get (Variables|Default|SetChar%20Ref _asbp_first_person_character))
    (Input|DisableInput _output_get (Game|GetPlayerController 0))
    (bind _alpha (Timeline|EnterPipe PlayFromStart)
      (:Update
        (Transformation|SetActorScale3D (Variables|Default|GetChar%20Ref) (Math|Conversions|ToVector(Float) (Math|Float|Lerp 1.0 0.1 _alpha))))
      (:Finished
        (bind _returnvalue (Actor|GetActorOfClass "/Game/_BPs/BP_PipeExit4.BP_PipeExit4_C"))
        (Variables|Default|SetNewVar_2 _returnvalue)
        (Variables|/Game/FirstPerson/Blueprints/BP_FirstPersonCharacter.BP_FirstPersonCharacter_C|SetExiting%20Pipe (Variables|Default|GetChar%20Ref) true)
        (Transformation|SetActorLocationAndRotation (Variables|Default|GetChar%20Ref) (Transformation|GetWorldLocation (Variables|/Game/_BPs/BP_PipeExit4.BP_PipeExit4_C|GetPipe2 (Variables|Default|GetNewVar_2))) (Transformation|GetWorldRotation (Variables|/Script/Engine.Actor|GetRootComponent (Variables|Default|GetNewVar_2))) false true)
        (bind _alpha_2 (Timeline|MoveUpFromTp PlayFromStart)
          (:Update
            (Transformation|SetActorScale3D (Variables|Default|GetChar%20Ref) (Math|Conversions|ToVector(Float) (Math|Float|Lerp 0.1 1.0 _alpha_2))))
          (:Finished
            (Input|EnableInput (Variables|Default|GetChar%20Ref) (Game|GetPlayerController 0))
            (Variables|/Game/FirstPerson/Blueprints/BP_FirstPersonCharacter.BP_FirstPersonCharacter_C|SetExiting%20Pipe (Variables|Default|GetChar%20Ref) false)))))))

(fn ConstructionScript)