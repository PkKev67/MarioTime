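; BP_LocalGravityAreaOLD is an unfinished local gravity volume, marked old by its name, that detects the first-person character.
; Overlap begin on GravArea, and every Tick while the player pawn overlaps it, calls GravityEvent.
; That event runs a debug-drawn component trace from Object toward the character's root against its capsule, leaving the result unused.
; The SetGravityDirection call is disconnected, so gravity never changes.
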(event OnComponentBeginOverlap(GravArea)
  (params (OverlappedComponent :type Primitive%20Component%20Object%20Reference) (OtherActor :type Actor%20Object%20Reference) (OtherComp :type Primitive%20Component%20Object%20Reference) (OtherBodyIndex :type Integer) (bFromSweep :type Boolean) (SweepResult :type Hit%20Result%20Structure%20%28by%20ref%29))
  (CallFunction|GravityEvent OtherActor))

(event OnComponentEndOverlap(GravArea)
  (params (OverlappedComponent :type Primitive%20Component%20Object%20Reference) (OtherActor :type Actor%20Object%20Reference) (OtherComp :type Primitive%20Component%20Object%20Reference) (OtherBodyIndex :type Integer)))

(event Custom|GravityEvent
  (params (HitObject :type Object%20Object%20Reference))
  (bind _asbp_first_person_character (Utilities|Casting|CastToBP_FirstPersonCharacter HitObject))
  (Collision|LineTraceComponent (Variables|/Script/Engine.Character|GetCapsuleComponent _asbp_first_person_character) (Transformation|GetWorldLocation (Variables|Default|GetObject)) (Transformation|GetWorldLocation (Variables|/Script/Engine.Actor|GetRootComponent _asbp_first_person_character)) true true false))

(event EventBeginPlay)

(event EventTick
  (params (DeltaSeconds :type Float%20%28single-precision%29))
  (bind _returnvalue (Game|Player|GetPlayerPawn 0))
  (if (Collision|IsOverlappingActor (Variables|Default|GetGravArea) _returnvalue :!class /Script/Engine.PrimitiveComponent)
    (CallFunction|GravityEvent _returnvalue)))

(fn ConstructionScript)