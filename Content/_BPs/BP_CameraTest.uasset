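; BP_CameraTest is a trigger actor that briefly switches the view to its own camera when the player enters its box.
; On overlap by BP_ThirdPersonCharacter, it deactivates the character's FollowCamera and activates its Camera component, then reverses both after a two-second delay.
; The switch toggles component activation, with debug prints at each step before the delay.
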(event OnComponentBeginOverlap(Box)
  (params (OverlappedComponent :type Primitive%20Component%20Object%20Reference) (OtherActor :type Actor%20Object%20Reference) (OtherComp :type Primitive%20Component%20Object%20Reference) (OtherBodyIndex :type Integer) (bFromSweep :type Boolean) (SweepResult :type Hit%20Result%20Structure%20%28by%20ref%29))
  (bind _asbp_third_person_character (Utilities|Casting|CastToBP_ThirdPersonCharacter OtherActor))
  (Development|PrintString "Casted")
  (Components|Activation|SetActive (Variables|/Game/Old+Unused/ThirdPerson/Blueprints/BP_ThirdPersonCharacter.BP_ThirdPersonCharacter_C|GetFollowCamera _asbp_third_person_character) false false)
  (Development|PrintString "Player cam deactiv")
  (Components|Activation|SetActive (Variables|Default|GetCamera) true false)
  (Development|PrintString "new cam active")
  (Utilities|FlowControl|Delay 2.0)
  (Components|Activation|SetActive (Variables|/Game/Old+Unused/ThirdPerson/Blueprints/BP_ThirdPersonCharacter.BP_ThirdPersonCharacter_C|GetFollowCamera _asbp_third_person_character) true false)
  (Components|Activation|SetActive (Variables|Default|GetCamera) false false))

(fn ConstructionScript)