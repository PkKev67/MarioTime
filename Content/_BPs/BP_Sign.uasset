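; BP_Sign is an interactable sign that shows and hides a placeholder text widget.
; Interact, gated by CanPressE and a CanInteract re-entry guard, flips InteractedWith to either create WBP_TextPlaceholder on the viewport or remove it.
; When BP_FirstPersonCharacter leaves the Sphere, the widget is removed and CanInteract re-enabled, but InteractedWith is not reset.
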(event OnComponentEndOverlap(Sphere)
  (params (OverlappedComponent :type Primitive%20Component%20Object%20Reference) (OtherActor :type Actor%20Object%20Reference) (OtherComp :type Primitive%20Component%20Object%20Reference) (OtherBodyIndex :type Integer))
  (bind _textwbp (Variables|Default|GetTextWBP))
  (Utilities|Casting|CastToBP_FirstPersonCharacter OtherActor)
  (if (Utilities|IsValid _textwbp)
    (Widget|RemovefromParent _textwbp))
  (Variables|Default|SetCanInteract true))

(event EventInteract
  (if (Variables|Default|GetCanPressE)
    (if (Variables|Default|GetCanInteract)
      (Variables|Default|SetCanInteract false)
      (if (Variables|Default|GetInteractedWith)
        (Variables|Default|SetInteractedWith false)
        (bind _returnvalue (UserInterface|CreateWidget "/Game/Interactables/WBP_TextPlaceholder.WBP_TextPlaceholder_C"))
        (bind _output_get (Variables|Default|SetTextWBP _returnvalue))
        (UserInterface|Viewport|AddtoViewport _output_get 0)
        (Variables|Default|SetCanInteract true)
        (else
          (Variables|Default|SetInteractedWith true)
          (if (Utilities|IsValid (Variables|Default|GetTextWBP))
            (Widget|RemovefromParent (Variables|Default|GetTextWBP)))
          (Variables|Default|SetCanInteract true))))))

(fn ConstructionScript
  (|CallParentFunction))